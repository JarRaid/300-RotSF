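; PrayerSpot is an interactable that fires a one-time trigger on a set of linked objects when the player interacts with it.
; The first interaction calls UpdateControlledObject and sets HasBeenTriggered to block repeats.
; That function sends TriggerMessage to each ControlledObjects entry implementing ITriggerOrToggle.
; Its lever-style toggle branch is disabled by a constant true condition, and Fix is an empty stub.
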(event EventPlayerWantstoInteract
  (params (PlayerCharacter :type Player%20Character%20Object%20Reference))
  (if (not (Variables|Default|GetHasBeenTriggered))
    (CallFunction|UpdateControlledObject)
    (Variables|Default|SetHasBeenTriggered true)))

(fn ConstructionScript)

(fn UpdateControlledObject
  (for _array_element (Variables|Default|GetControlled%20Objects)
    (if (Utilities|DoesObjectImplementInterface _array_element "/Game/Blueprints/Interface/ITriggerOrToggle.ITriggerOrToggle_C")
      (if true
        (Class|ITriggerorToggle|Trigger(Message) _array_element)
        (else
          (Class|ITriggerorToggle|Toggle(Message) _array_element (Variables|Default|GetIsLeverOn)))))))

(fn Fix
  (params (Currently%20held%20item :type Actor%20Object%20Reference)))