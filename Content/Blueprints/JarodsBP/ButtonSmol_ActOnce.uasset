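; Small push-button actor that the player operates with Interact to signal a list of controlled objects.
; Its Box overlap enables input when a PlayerCharacter enters; any end overlap disables it.
; Interact plays a sound and restarts a timeline that slides ButtonMover along X.
; Every timeline update sends IsPressed, never set here, via ToggleMessage to ControlledObjects implementing ITriggerOrToggle; despite the ActOnce name, nothing blocks repeat presses.
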(event OnComponentBeginOverlap(Box)
  (params (OverlappedComponent :type Primitive%20Component%20Object%20Reference) (OtherActor :type Actor%20Object%20Reference) (OtherComp :type Primitive%20Component%20Object%20Reference) (OtherBodyIndex :type Integer) (bFromSweep :type Boolean) (SweepResult :type Hit%20Result%20Structure%20%28by%20ref%29))
  (Utilities|Casting|CastToPlayerCharacter OtherActor)
  (Input|EnableInput (Game|GetPlayerController 0)))

(event OnComponentEndOverlap(Box)
  (params (OverlappedComponent :type Primitive%20Component%20Object%20Reference) (OtherActor :type Actor%20Object%20Reference) (OtherComp :type Primitive%20Component%20Object%20Reference) (OtherBodyIndex :type Integer))
  (Input|DisableInput (Game|GetPlayerController 0)))

(event EventBeginPlay)

(event Collision|EventActorBeginOverlap
  (params (OtherActor :type Actor%20Object%20Reference)))

(event EventTick
  (params (DeltaSeconds :type Float%20%28single-precision%29)))

(event Input|ActionEvents|InputActionInteract
  (params (Key :type Key%20Structure :default "None"))
  (:Pressed
    (Audio|PlaySoundatLocation "/Game/Audio/JarodsAudio/ButtonGranted.ButtonGranted" (Transformation|GetActorLocation) "0, 0, 0" 1.0 1.0 0.0 0 0 0)
    (bind _translate (Timeline|ButtonAnim PlayFromStart)
      (:Update
        (Transformation|SetRelativeLocation (Variables|Default|GetButtonMover) (Math|Vector|MakeVector (.x _translate) 0.0 0.0) false false)
        (CallFunction|UpdateControlledObjects)))))

(fn ConstructionScript)

(fn UpdateControlledObjects
  (for _array_element (Variables|Default|GetControlledObjects)
    (if (Utilities|DoesObjectImplementInterface _array_element "/Game/Blueprints/Interface/ITriggerOrToggle.ITriggerOrToggle_C")
      (Class|ITriggerorToggle|Toggle(Message) _array_element (Variables|Default|GetIsPressed)))))