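; LeverOnce is a single-use interactable lever that toggles or triggers its controlled objects through the ITriggerOrToggle interface.
; The first interaction sets HasBeen, even on a broken lever, and blocks later ones.
; A working lever flips its state, messages its targets and rotates its hinge by timeline, springing back in trigger mode.
; Broken levers hide their mesh until Fix receives a held item that repairs levers.
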(event EventPlayerWantstoInteract
  (params (PlayerCharacter :type Player%20Character%20Object%20Reference))
  (if (not (Variables|Default|GetHasBeen))
    (Variables|Default|SetHasBeen true)
    (Components|Timeline|SetPlayRate (Variables|Default|GetThrow%20The%20Lever!) (select (Variables|Default|GetIs%20a%20trigger) 2.0 1.0))
    (if (not (Variables|Default|GetIsLeverBroken))
      (Variables|Default|SetIsLeverOn (not (Variables|Default|GetIsLeverOn)))
      (CallFunction|UpdateControlledObject)
      (if (or (Variables|Default|GetIsLeverOn) (Variables|Default|GetIs%20a%20trigger))
        (bind (_direction _hinge_rotation_y) (Timeline|Throw%20The%20Lever! Play)
          (:Update
            (Transformation|SetRelativeRotation (Variables|Default|GetHinge) (Math|Rotator|MakeRotator 0.0 (* _hinge_rotation_y (Variables|Default|GetAngle%20to%20rotate)) 0.0) false false))
          (:Finished
            (if (and (Utilities|Enum|Equal(Enum) _direction "Forward") (Variables|Default|GetIs%20a%20trigger))
              (Timeline|Throw%20The%20Lever! Reverse))))
        (else
          (Timeline|Throw%20The%20Lever! Reverse))))))

(event EventBeginPlay
  (Variables|Default|SetHasBeen false)
  (bind (_direction _hinge_rotation_y) (Timeline|Throw%20The%20Lever! SetNewTime)
    (:Update
      (Transformation|SetRelativeRotation (Variables|Default|GetHinge) (Math|Rotator|MakeRotator 0.0 (* _hinge_rotation_y (Variables|Default|GetAngle%20to%20rotate)) 0.0) false false))
    (:Finished
      (if (and (Utilities|Enum|Equal(Enum) _direction "Forward") (Variables|Default|GetIs%20a%20trigger))
        (Timeline|Throw%20The%20Lever! Reverse)))))

(fn ConstructionScript
  (Rendering|SetVisibility (Variables|Default|GetMesh%20-%20Lever) (not (Variables|Default|GetIsLeverBroken)) false)
  (Transformation|SetRelativeRotation (Variables|Default|GetHinge) (Math|Rotator|MakeRotator 0.0 (* (Variables|Default|GetAngle%20to%20rotate) (select (Variables|Default|GetIsLeverOn) 1.0 -1.0)) 0.0) false false))

(fn UpdateControlledObject
  (for _array_element (Variables|Default|GetControlled%20Objects)
    (if (Utilities|DoesObjectImplementInterface _array_element "/Game/Blueprints/Interface/ITriggerOrToggle.ITriggerOrToggle_C")
      (if (Variables|Default|GetIs%20a%20trigger)
        (Class|ITriggerorToggle|Trigger(Message) _array_element)
        (else
          (Class|ITriggerorToggle|Toggle(Message) _array_element (Variables|Default|GetIsLeverOn)))))))

(fn Fix
  (params (Currently%20held%20item :type Actor%20Object%20Reference))
  (bind _aspickupable_object (Utilities|Casting|CastToPickupableObject Currently%20held%20item)
    (:then
      (if (Variables|/Game/Blueprints/PickupableObject.PickupableObject_C|GetFixes%20levers _aspickupable_object)
        (if (Variables|Default|GetIsLeverBroken)
          (Variables|Default|SetIsLeverBroken false)
          (Rendering|SetVisibility (Variables|Default|GetMesh%20-%20Lever) true false)
          (return true)
          (else
            _))))
    (:CastFailed
      _))
  (return false))